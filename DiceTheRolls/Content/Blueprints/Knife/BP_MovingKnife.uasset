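; Moving knife actor that slides between two points offset from its placed location and pauses while its Chopping flag is set.
; On BeginPlay it stores that location and assigns itself to BP_PlayerController's Knife reference.
; Tick drives the lerp through KnifeCurve, sampled on looping time with a period set by SecondsPerSection and the ChoppingSections count.
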(event `self.ReceiveTick`
  (params (DeltaSeconds :type "Float (single-precision)"))
  (bind _originallocation (`self.OriginalLocation`))
  (if (not (`self.Chopping`))
    (bind _output_get (set `self.DeltaSeconds` (+ DeltaSeconds (`self.DeltaSeconds`))))
    (`self.K2_SetActorLocation` (`KismetMathLibrary.VLerp` (+ (`self.StartPoint`) _originallocation) (+ _originallocation (`self.EndPoint`)) (`CurveFloat.GetFloatValue` (`self.KnifeCurve`) (mod (/ _output_get (* (`self.SecondsPerSection`) (+ (`self.ChoppingSections`) 1))) 1.0))))))

(event `self.ReceiveBeginPlay`
  (`parent.ReceiveBeginPlay`)
  (set `self.OriginalLocation` (`self.K2_GetActorLocation`))
  (bind _asbp_player_controller (cast `/Game/Blueprints/BP_PlayerController` (`GameplayStatics.GetPlayerController` 0)))
  (set `/Game/Blueprints/BP_PlayerController.Knife` self _asbp_player_controller))

(fn `UserConstructionScript`
  (`parent.UserConstructionScript`))