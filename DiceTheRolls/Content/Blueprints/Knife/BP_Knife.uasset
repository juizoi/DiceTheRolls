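; Player knife for a food-chopping game, which slices the spawner's current item and scores each cut.
; Chop traces down from the socket for the procedural component, plays a montage, slices on its notify with camera shake, and respawns the item at the chop limit.
; Box overlaps score each new hit box once, using its width to pick the good or bad cut sound; both award equal points.
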(event `ClearArrays`
  (`KismetArrayLibrary.Array_Clear` (`self.HitActors`))
  (`KismetArrayLibrary.Array_Clear` (`self.HitComponents`)))

(event `Chop`
  (bind _procedural_component (`self.Procedural Component`))
  (bind _returnvalue (`SceneComponent.K2_GetComponentLocation` (`self.Socket`)))
  (if (not (`self.Chopping`))
    (bind _outhit (`KismetSystemLibrary.LineTraceSingle` :`Start` _returnvalue :`End` (`KismetMathLibrary.MakeVector` (.x _returnvalue) (.y _returnvalue) (- (.z _returnvalue) 1000.0)) :`TraceChannel` "TraceTypeQuery1" :`DrawTime` 400.0))
    (bind _output_get (set `self.Procedural Component` (`.HitComponent` (`GameplayStatics.BreakHitResult` _outhit))))
    (set `self.Chopping` true)
    (`|PlayMontage` (`self.KnifeMesh`) "/Game/Assets/Animations/Knife/SK_Knife_Skeleton_Montage.SK_Knife_Skeleton_Montage"
      (:`OnCompleted`
        (set `self.Chopping` false)
        (`/Engine/EditorBlueprintResources/StandardMacros.IsValid` _output_get :!label _label
          (:`Is Valid`
            (bind _result (`/Engine/EditorBlueprintResources/StandardMacros.IncrementInt` (`self.ChopCounter`))
              (:`  `
                (if (== _result (`self.MaxNumChops`))
                  (`/Game/Blueprints/Spawner/BP_ItemSpawner.Respawn` (`self.Spawner`))
                  (set `self.ChopCounter` 0)))))
          (:`Is Not Valid`
            (`KismetSystemLibrary.Delay` 0.05)
            (`GameplayStatics.PlaySound2D` "/Game/Sounds/MissedCut.MissedCut" 1.0 1.0 0.0 null null))))
      (:`OnInterrupted`
        (goto _label))
      (:`OnNotifyBegin`
        (bind _currentitem (`/Game/Blueprints/Spawner/BP_ItemSpawner.CurrentItem` (`self.Spawner`))
          (:`then`
            (`KismetSystemLibrary.PrintString` (`KismetSystemLibrary.GetDisplayName` _procedural_component))
            (`/Game/Blueprints/BP_BaseItem.Slice` _currentitem _procedural_component)
            (`GameplayStatics.PlayWorldCameraShake` "/Game/Effects/BP_ChopShake.BP_ChopShake_C" (`self.K2_GetActorLocation`) 0.0 500.0))
          (:`else`))))))

(event `self.Box.OnComponentBeginOverlap`
  (params (OverlappedComponent :type "PrimitiveComponent Object Reference") (OtherActor :type "Actor Object Reference") (OtherComp :type "PrimitiveComponent Object Reference") (OtherBodyIndex :type Integer) (bFromSweep :type Boolean) (SweepResult :type "HitResult Structure (by ref)"))
  (bind _alreadyhitboxes (`self.AlreadyHitBoxes`))
  (if (!= OtherComp (`self.Box`))
    (bind _asbox_collision (cast `BoxComponent` OtherComp))
    (if (not (`KismetArrayLibrary.Array_Contains` _alreadyhitboxes _asbox_collision))
      (`KismetArrayLibrary.Array_Add` _alreadyhitboxes _asbox_collision)
      (bind _gameinstanceref (`self.GameInstanceRef`)
        (:`then`
          (bind _boxextent_x (`KismetMathLibrary.BreakVector` (`BoxComponent.BoxExtent` _asbox_collision)))
          (if (> _boxextent_x 0.2)
            ;[1 1 1] Bad Cut
            (`/Game/Blueprints/GI_DiceTheRoll.IncrementScore` _gameinstanceref 25)
            (`GameplayStatics.PlaySound2D` "/Game/Sounds/CutFoodGeneric.CutFoodGeneric" 1.0 1.0 0.0 null null)
            (else
              ;[1 1 1] Good Cut
              (`/Game/Blueprints/GI_DiceTheRoll.IncrementScore` _gameinstanceref 25)
              (`GameplayStatics.PlaySound2D` "/Game/Sounds/PerfectCue.PerfectCue" 1.0 1.0 0.0 null null))))
        (:`else`)))))

(event `self.ReceiveBeginPlay`
  (bind _asgi_dice_the_roll (cast `/Game/Blueprints/GI_DiceTheRoll` (`GameplayStatics.GetGameInstance`)))
  (set `self.GameInstanceRef` _asgi_dice_the_roll))

(fn `UserConstructionScript`)