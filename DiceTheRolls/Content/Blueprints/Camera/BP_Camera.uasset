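; BP_Camera is a possessable camera rig with a spring arm that zooms when play starts via its PlayGame event.
; On BeginPlay it has player controller 0 possess it, and the construction script sets the arm length from its TargetArmLength variable.
; PlayGame runs the Zoom timeline, which lerps the arm from that length to a fixed final distance.
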(event `self.ReceiveBeginPlay`
  (`Controller.Possess` (`GameplayStatics.GetPlayerController` 0) self))

(event `Play Game`
  (bind (_direction _zoomalpha) (`Timeline|Zoom`)
    (:`Update`
      (set `SpringArmComponent.TargetArmLength` (`KismetMathLibrary.Lerp` (`self.Target Arm Length`) 400.0 _zoomalpha) (`self.SpringArm`)))))

(fn `UserConstructionScript`
  (set `SpringArmComponent.TargetArmLength` (`self.Target Arm Length`) (`self.SpringArm`)))