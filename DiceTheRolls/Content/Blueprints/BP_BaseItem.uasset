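; Base item that the knife slices into pieces, with evenly spaced guides marking the target cuts.
; Construction script places box components and indicator meshes along the mesh's X bounds and records cut locations.
; BeginPlay swaps the static mesh for a procedural copy; Slice cuts every piece at the knife's plane, nudging pieces apart by side.
; OldGetScore only prints whether a piece's size is within threshold.
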(event `SeparatePieces`
  (params (`HitComponents ` :type "Array of ProceduralMeshComponent Object Reference"))
  (for _array_element `HitComponents `
    (bind _relativelocation_x (`KismetMathLibrary.BreakVector` (`SceneComponent.RelativeLocation` _array_element)))
    (`SceneComponent.K2_AddLocalOffset` _array_element (`KismetMathLibrary.MakeVector` (+ _relativelocation_x -1.0)) false false)))

(event `self.ReceiveBeginPlay`
  (bind _mesh (`self.Mesh`))
  (bind _proceduralmesh (`self.ProceduralMesh`))
  (`KismetProceduralMeshLibrary.CopyProceduralMeshFromStaticMeshComponent` _mesh 0 _proceduralmesh true)
  (`SceneComponent.K2_SetRelativeTransform` _proceduralmesh (`SceneComponent.GetRelativeTransform` _mesh) false false)
  (`KismetArrayLibrary.Array_Set` (`self.ProceduralMeshNet`) 0 _proceduralmesh true)
  (`ActorComponent.K2_DestroyComponent` _mesh))

(event `Slice`
  (params (InComp :type "SceneComponent Object Reference"))
  (for _array_element (`self.ProceduralMeshNet`)
    (bind _outotherhalfprocmesh (`KismetProceduralMeshLibrary.SliceProceduralMesh` _array_element (`SceneComponent.K2_GetComponentLocation` (`/Game/Blueprints/Knife/BP_Knife.KnifeMesh` (`self.KnifeRef`))) (0.0 1.0 0.0) true "CreateNewSectionForCap" "/Game/StarterContent/Materials/M_Brick_Clay_New.M_Brick_Clay_New"))
    (`SceneComponent.K2_AttachToComponent` _outotherhalfprocmesh (`self.ProceduralMeshes`) "None" "KeepWorld" "KeepWorld" "KeepWorld" false)
    (`KismetArrayLibrary.Array_Add` (`self.tempProceduralMeshNet`) _outotherhalfprocmesh))
  (for _array_element_2 (`self.ProceduralMeshNet`)
    (`SceneComponent.K2_AddLocalOffset` _array_element_2 (`KismetMathLibrary.MakeVector` (* (- 1.0 (`KismetMathLibrary.SignOfFloat` (- (.y (`self.K2_GetActorLocation` (`self.KnifeRef`))) (.y (`KismetSystemLibrary.GetComponentBounds` _array_element_2))))) 0.1)) false false))
  (`KismetArrayLibrary.Array_Append` (`self.ProceduralMeshNet`) (`self.tempProceduralMeshNet`))
  (`KismetArrayLibrary.Array_Clear` (`self.tempProceduralMeshNet`)))

(fn `UserConstructionScript`
  (bind _mesh (`self.Mesh`))
  (bind (_min _max) (break `Box` (`StaticMesh.GetBoundingBox` (`StaticMeshComponent.StaticMesh` _mesh))))
  (`|ExecutionSequence`
    (:`then_0`
      (for _array_element (`SceneComponent.GetChildrenComponents` (`self.IndicatorParent`) false)
        (`ActorComponent.K2_DestroyComponent` _array_element)))
    (:`then_1`
      (`/Engine/EditorBlueprintResources/StandardMacros.IsValid` _mesh
        (:`Is Valid`
          (for _index (range 1 (+ (`self.Cuts`) 1))
            (bind _returnvalue (`KismetMathLibrary.MakeVector` (`KismetMathLibrary.Lerp` (.x _min) (.x _max) (/ _index (+ (`self.Cuts`) 1)))))
            (`BlueprintMapLibrary.Map_Add` (`self.CutLocations`) _index _returnvalue)
            (`AddComponent|NODE_AddBoxComponent-1` :`RelativeTransform` (`KismetMathLibrary.MakeTransform` _returnvalue (struct) (3.0 1.0 1.0)))
            (`AddComponent|NODE_AddBoxComponent-2` :`RelativeTransform` (`KismetMathLibrary.MakeTransform` _returnvalue (struct) (3.0 1.0 1.0)))
            (bind _returnvalue_2 (`AddComponent|NODE_AddStaticMeshComponent-0` :`RelativeTransform` (`KismetMathLibrary.MakeTransform` _returnvalue (struct) (3.0 1.0 1.0))))
            (`StaticMeshComponent.SetStaticMesh` _returnvalue_2 "/Game/Assets/Roll/SM_Indicator.SM_Indicator")
            (`PrimitiveComponent.SetCastShadow` _returnvalue_2 false)
            (`SceneComponent.K2_AttachToComponent` _returnvalue_2 (`self.IndicatorParent`) "None" "KeepRelative" "KeepRelative" "KeepRelative" false)))))))