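; BP_ItemSpawner is an item spawner that places an item at its own transform on BeginPlay and respawns it on demand.
; It spawns the first class in ItemsToSpawn only when no CurrentItem exists, passing its KnifeRef to the new item.
; Respawn destroys the current item, clears the knife's arrays, then waits a configurable delay before spawning again.
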(event `self.ReceiveBeginPlay`
  (`self.AttemptToSpawn` :!label _label))

(event `Respawn`
  (bind _currentitem (`self.CurrentItem`)
    (:`then`
      (`self.K2_DestroyActor` _currentitem))
    (:`else`
      _))
  (`/Game/Blueprints/Knife/BP_Knife.ClearArrays` (`self.KnifeRef`))
  (set `self.CurrentItem` null)
  (`KismetSystemLibrary.Delay` (`self.DelayBeforeRespawn`))
  (goto _label))

(fn `AttemptToSpawn`
  (`/Engine/EditorBlueprintResources/StandardMacros.IsValid` (`self.CurrentItem`)
    (:`Is Valid`
      (`KismetSystemLibrary.PrintString` "Item already Spawned"))
    (:`Is Not Valid`
      (`self.SpawnItem`))))

(fn `SpawnItem`
  (bind _returnvalue (`|SpawnActorFromClass` (`|GetArrayItem` (`self.ItemsToSpawn`)) (`KismetMathLibrary.MakeTransform` (`self.K2_GetActorLocation`) (`self.K2_GetActorRotation`)) "AdjustIfPossibleButAlwaysSpawn" "OverrideRootScale" self null))
  (set `/Game/Blueprints/BP_BaseItem.KnifeRef` (`self.KnifeRef`) _returnvalue)
  (set `self.CurrentItem` _returnvalue))

(fn `UserConstructionScript`)